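; BP_Map02 is a Map02 actor whose CameraBoeder collision component tells the player character when it is inside a camera border.
; When an actor tagged Player begins overlapping, it gets the character reference from player pawn 0 through an interface call, stores the pawn's location as CameraBorderLocation and sets InBorder.
; When the overlap ends, it clears InBorder; camera behavior itself is not handled here.
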(event OnComponentBeginOverlap(CameraBoeder)
  (params (OverlappedComponent :type Primitive%20Component%20Object%20Reference) (OtherActor :type Actor%20Object%20Reference) (OtherComp :type Primitive%20Component%20Object%20Reference) (OtherBodyIndex :type Integer) (bFromSweep :type Boolean) (SweepResult :type Hit%20Result%20Structure%20%28by%20ref%29))
  (bind _returnvalue (Game|Player|GetPlayerPawn 0))
  (if (Actor|ActorHasTag OtherActor "Player")
    (bind _characterref (Class|BPICharacter|BPIGetCharacterRef(Message) _returnvalue))
    (Variables|/Game/_Game_/GamePaly/BP_/Player/BP_Character.BP_Character_C|SetCameraBorderLocation _characterref (Transformation|GetActorLocation _returnvalue))
    (Variables|/Game/_Game_/GamePaly/BP_/Player/BP_Character.BP_Character_C|SetInBorder _characterref true)))

(event OnComponentEndOverlap(CameraBoeder)
  (params (OverlappedComponent :type Primitive%20Component%20Object%20Reference) (OtherActor :type Actor%20Object%20Reference) (OtherComp :type Primitive%20Component%20Object%20Reference) (OtherBodyIndex :type Integer))
  (if (Actor|ActorHasTag OtherActor "Player")
    (bind _characterref (Class|BPICharacter|BPIGetCharacterRef(Message) (Game|Player|GetPlayerPawn 0)))
    (Variables|/Game/_Game_/GamePaly/BP_/Player/BP_Character.BP_Character_C|SetInBorder _characterref false)))

(fn ConstructionScript)