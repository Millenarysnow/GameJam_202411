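; Player character for a flipbook side-view puzzle game where sleeping at a bed switches between reality and a dream Painting view.
; In reality it walks, jumps, flies with a parachute item and interacts with doors, ropes and pickups through a key inventory.
; In the dream, mouse clicks collect keys and queue a limited set of platforms that decide which show on waking.
; A spawned orthographic camera eases position and width per view.
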(event Custom|SpawnCamera
  ;[1 1 1] BeginPlay
  (bind _returnvalue (Game|SpawnActorfromClass "/Game/_Game_/GamePaly/BP_/Camera/BP_Camera.BP_Camera_C" (Math|Transform|MakeTransform (+ (Transformation|GetActorLocation) "0.000000,0.000000,500.000000") "0, 0, 0" "1.000000,1.000000,1.000000") "Undefined" "MultiplyWithRoot" 0 0))
  (bind _output_get (Variables|Camera|SetCameraRef _returnvalue))
  (Utilities|IsValid _output_get
    (:Is%20Valid
      (bind _cameraref (Variables|Camera|GetCameraRef)
        (:then
          (Game|Player|SetViewTargetwithBlend (Variables|PC|GetPC) _cameraref 0.0 "VTBlend_Linear" 0.0 false))
        (:else)))))

(event Custom|GetPalyerController
  ;[1 1 1] BeginPlay
  (Variables|PC|SetPC (Game|GetPlayerController 0))
  (Variables|Camera|SetCameraRootLocation (Transformation|GetActorLocation)))

(event Custom|UpdateCameraLocation
  (bind _returnvalue (Transformation|GetActorLocation))
  (bind _cameraborderlocation (Variables|摄像机|GetCameraBorderLocation))
  (bind _cameraoffest (Variables|摄像机|GetCameraOffest))
  (bind _cameraoffest_2 (Variables|摄像机|GetCameraOffest))
  (bind _camerarootlocation (Variables|Camera|GetCameraRootLocation))
  (bind _cameraoffest_3 (Variables|摄像机|GetCameraOffest))
  (bind _zooming (Variables|摄像机|GetZooming))
  (bind _view (Variables|摄像机|GetView))
  (bind _cameralocation (Variables|摄像机|GetCameraLocation))
  (bind _camerarootlocation_2 (Variables|Camera|GetCameraRootLocation))
  (bind _paintingviewlocation (Variables|摄像机|GetPaintingViewLocation))
  (bind _inborder (Variables|摄像机|GetInBorder))
  (bind (_x _y) (Math|Vector|BreakVector _returnvalue))
  (bind _returnvalue_2 (+ _cameraborderlocation _cameraoffest))
  (bind _returnvalue_3 (+ _camerarootlocation_2 _cameraoffest_2))
  (bind _returnvalue_4 (+ _camerarootlocation _cameraoffest_3))
  (bind _returnvalue_5 (select _zooming _cameralocation _paintingviewlocation))
  (bind _z (Math|Vector|BreakVector _returnvalue_3))
  (bind (_x_2 _y_2) (Math|Vector|BreakVector _returnvalue_2))
  (bind _z_2 (Math|Vector|BreakVector _returnvalue_4))
  (bind _returnvalue_6 (Math|Vector|MakeVector _x _y _z_2))
  (bind _returnvalue_7 (Math|Vector|MakeVector _x_2 _y_2 _z))
  (bind _returnvalue_8 (Utilities|Select :Index _view :NewEnumerator0 _returnvalue_5 :NewEnumerator1 _returnvalue_6 :NewEnumerator2 "0, 0, 0"))
  (bind _returnvalue_9 (select _inborder _returnvalue_7 _returnvalue_8))
  ;[1 1 1] Tick
  (bind _cameraline (Timeline|CameraMove PlayFromStart)
    (:Update
      (bind _cameraref (Variables|Camera|GetCameraRef)
        (:then
          (Transformation|SetActorLocation _cameraref (Math|Vector|Lerp(Vector) (Transformation|GetActorLocation (Variables|Camera|GetCameraRef)) (Utilities|Select :Index (Variables|摄像机|GetView) :NewEnumerator0 _returnvalue_9 :NewEnumerator1 _returnvalue_9 :NewEnumerator2 (Variables|摄像机|GetOverallCameraLocation)) _cameraline) false false)
          (bind _output_get (Variables|摄像机|SetCameraFov (Math|Float|Lerp (Variables|摄像机|GetCameraFov) (Utilities|Select :Index (Variables|摄像机|GetView) :NewEnumerator0 (Variables|摄像机|GetPaintingView) :NewEnumerator1 (Variables|摄像机|GetChatacterView) :NewEnumerator2 2048.0) _cameraline)))
          (Class|CameraComponent|SetOrthoWidth (Variables|/Game/_Game_/GamePaly/BP_/Camera/BP_Camera.BP_Camera_C|GetCamera _cameraref) _output_get))
        (:else)))))

(event Custom|AddMapping
  (bind _pc (Variables|PC|GetPC))
  (bind _returnvalue (PlayerController|LocalPlayerSubsystems|GetEnhancedInputLocalPlayerSubsystem _pc))
  ;[1 1 1] BeginPlay
  ;;[1 0 0] 暂留
  (Utilities|IsValid _returnvalue
    (:Is%20Valid
      (Input|AddMappingContext _returnvalue "/Game/_Game_/GamePaly/Dream_IM.Dream_IM" 0 "(bIgnoreAllPressedKeysUntilRelease=True,bForceImmediately=False,bNotifyUserSettings=False)"))))

(event Custom|Switch%20CanFly
  ;[1 1 1] Switch status fly
  (if (Variables|Input|GetIsFlying)
    _))

(event Custom|StartFly
  ;[1 1 1] Switch status fly
  (if (CallFunction|FindBackKeys (Variables|Interact|Getkeys) 6 true)
    (Variables|Input|SetIsFlying true)
    (Pawn|Components|CharacterMovement|SetMovementMode (Variables|Character|GetCharacterMovement) "MOVE_Flying" 0)
    (Variables|Movement|SetMovementState "NewEnumerator2")
    (Audio|PlaySound2D "/Game/_Game_/Audio/SFX/object/para/SC_paraUse.SC_paraUse" 1.0 1.0 0.0 0 0)
    (Rendering|SetVisibility (Variables|Default|GetT_jiangluosan1) true false)))

(event Custom|EndFly
  ;[1 1 1] Switch status fly
  (if (CallFunction|FindBackKeys (Variables|Interact|Getkeys) 6 true)
    (Variables|Input|SetIsFlying false)
    (Pawn|Components|CharacterMovement|SetMovementMode (Variables|Character|GetCharacterMovement) "MOVE_NavWalking" 0)
    (Rendering|SetVisibility (Variables|Default|GetT_jiangluosan1) false false)))

(event EventBeginPlay
  (Utilities|FlowControl|Sequence
    (:then_0
      (CallFunction|GetPalyerController)
      (CallFunction|SpawnCamera)
      (CallFunction|AddMapping))
    (:then_1
      (CallFunction|CreatBackpackUI))))

(event EventTick
  (params (DeltaSeconds :type Float%20%28single-precision%29))
  (Utilities|FlowControl|Sequence
    (:then_0
      (CallFunction|UpdateCameraLocation))))

(event Custom|Move
  (params (ActionValue :type Float%20%28double-precision%29))
  ;[1 1 1] IA_move
  (if (not (Variables|Default|GetInDelay))
    (switch Utilities|FlowControl|Switch|SwitchonE_View (Variables|摄像机|GetView)
      (:NewEnumerator1
        _)
      (:NewEnumerator2
        _))
    (if (Variables|Input|GetIsFlying)
      (if (Variables|Input|GetIsFlying)
        (Transformation|AddActorLocalOffset (Math|Vector|MakeVector 0.0 0.0 3.0) true false))
      (Variables|Movement|SetMovementState (select (< ActionValue 0.0) "NewEnumerator0" (select (> ActionValue 0.0) "NewEnumerator1" "NewEnumerator4")) :!label _label)
      (elif (== (.z (Variables|/Script/Engine.MovementComponent|GetVelocity (Variables|Character|GetCharacterMovement))) 0.0)
        (goto _label)
        (else
          (Variables|Movement|SetMovementState "NewEnumerator2"))))
    (switch Utilities|FlowControl|Switch|SwitchonE_MovementState (Variables|Movement|GetMovementState)
      (:NewEnumerator4
        (CallFunction|StopWalkSound)
        (Pawn|Input|AddMovementInput (Math|Vector|GetForwardVector (Variables|Default|GetDirection)) (Input|AxisValues|GetMove) true :!label _label_2))
      (:NewEnumerator0
        (CallFunction|PlayWalkSound :!label _label_3)
        (goto _label_2))
      (:NewEnumerator1
        (goto _label_3))
      (:NewEnumerator2
        (CallFunction|StopWalkSound)
        (Pawn|Input|AddMovementInput (Math|Vector|GetForwardVector (Variables|Default|GetDirection)) (Input|AxisValues|GetMove) true)))))

(event Custom|Interact
  ;[1 1 1] Sleep
  (switch Utilities|FlowControl|Switch|SwitchonE_Interact (Variables|Interact|GetInteractState)
    (:NewEnumerator0
      (if (Variables|Interact|GetCanInteract)
        (Variables|Interact|SetCanInteract true)
        (switch Utilities|FlowControl|Switch|SwitchonE_View (Variables|摄像机|GetView)
          (:NewEnumerator0
            (CallFunction|SoundsAboutDreamtoReality)
            (Utilities|FlowControl|Sequence
              (:then_0
                (Variables|摄像机|SetZooming false)
                (Variables|摄像机|SetPaintingView 1.8e+03))
              (:then_1
                (Variables|摄像机|SetView "NewEnumerator1")
                (Utilities|FlowControl|Sequence
                  (:then_0
                    (Variables|/Script/Engine.PlayerController|SetbShowMouseCursor (Variables|PC|GetPC) false)
                    (bind _outactors (Actor|GetAllActorsOfClass "/Game/_Game_/GamePaly/BP_/Others/BP_Traps.BP_Traps_C"))
                    (for _array_element _outactors
                      (if (Actor|ActorHasTag _array_element "Trap")
                        (bind _trapref (Class|BPITraps|BPIGetTrapRef(Message) _array_element))
                        (Default|SetMaterial _trapref false)))
                    (Default|OutDreamCalledbyCharacterBP (Variables|UI|GetDream_UI))
                    (Variables|Interact|SetCanInteract true))
                  (:then_1
                    (bind _outactors_2 (Actor|GetAllActorsOfClass "/Game/_Game_/GamePaly/BP_/Others/BP_Platform.BP_Platform_C"))
                    (for _array_element_2 _outactors_2
                      (if (Utilities|Array|ContainsItem (Variables|Default|GetPlatformsRef) _array_element_2)
                        (Default|ShowPlatformCalledbyCharacterBP _array_element_2)
                        (else
                          (Default|HidePlatformCalledbyCharacterBP _array_element_2)))))))))
          (:NewEnumerator1
            (if (Variables|Input|GetCanSleep)
              (CallFunction|InSleep)
              (Utilities|EffectRealitytoDream)
              (Utilities|FlowControl|Sequence
                (:then_0
                  (Variables|摄像机|SetView "NewEnumerator0")
                  (Variables|/Script/Engine.PlayerController|SetbShowMouseCursor (Variables|PC|GetPC) true)
                  (bind _outactors_3 (Actor|GetAllActorsOfClass "/Game/_Game_/GamePaly/BP_/Others/BP_Traps.BP_Traps_C"))
                  (for _array_element_3 _outactors_3
                    (if (Actor|ActorHasTag _array_element_3 "Trap")
                      (bind _trapref_2 (Class|BPITraps|BPIGetTrapRef(Message) _array_element_3))
                      (Default|SetMaterial _trapref_2 true)))
                  (Default|EnterDreamCalledbyCharacterBP (Variables|UI|GetDream_UI))
                  (Variables|Interact|SetCanInteract true))
                (:then_1
                  (bind _outactors_4 (Actor|GetAllActorsOfClass "/Game/_Game_/GamePaly/BP_/Others/BP_Platform.BP_Platform_C"))
                  (for _array_element_4 _outactors_4
                    (Default|ShowAll _array_element_4)))))))))
    (:NewEnumerator1
      (switch Utilities|FlowControl|Switch|SwitchonE_View (Variables|摄像机|GetView)
        (:NewEnumerator1
          (if (Variables|interact|GetinDoor)
            (bind _doorref (Variables|Interact|GetDoorRef)
              (:then
                (Default|InteractCalledbyCharacterBP _doorref (CallFunction|FindBackKeys (Variables|Interact|Getkeys) (Variables|/Game/_Game_/GamePaly/BP_/Others/BP_Door01.BP_Door01_C|GetDoorindex_Key _doorref) false)))
              (:else))))))
    (:NewEnumerator2
      (if (Variables|Interact|GetInTransDoor)
        (bind _transdoorref (Variables|Interact|GetTransDoorRef)
          (:then
            (Default|TransPlayer _transdoorref))
          (:else))))
    (:NewEnumerator3
      (if (Variables|Interact|GetInRope)
        (bind _bridgeref (Variables|Interact|GetBridgeRef)
          (:then
            (if (CallFunction|FindBackKeys (Variables|Interact|Getkeys) (Variables|/Game/_Game_/GamePaly/BP_/Others/BP_Bridge.BP_Bridge_C|Getindex _bridgeref) true)
              (Default|CutRope _bridgeref)))
          (:else))))
    (:NewEnumerator4
      (if (Variables|Interact|GetCanPick)
        (bind _tool (Variables|Interact|GetTool)
          (:then
            (Default|PlayPickupSFX _tool)
            (Utilities|Array|AddUnique (Variables|Interact|Getkeys) (Utilities|Struct|MakeST_key (Variables|/Game/_Game_/GamePaly/BP_/Others/BP_Tool.BP_Tool_C|Getindex _tool) (Variables|/Game/_Game_/GamePaly/BP_/Others/BP_Tool.BP_Tool_C|GetImage _tool)))
            (Actor|DestroyActor _tool)
            (Variables|Interact|SetTool 0)
            (Default|RefreshUI (Variables|UI|GetBackpackUI) (Variables|Interact|Getkeys)))
          (:else))))))

(event Custom|Painting_Event
  (bind (_hit _actor) (CallFunction|CheckHit "Platform"))
  (bind (_hit_2 _actor_2) (CallFunction|CheckHit "Key"))
  ;[1 1 1] LeftMouseClick
  (switch Utilities|FlowControl|Switch|SwitchonE_View (Variables|摄像机|GetView)
    (:NewEnumerator0
      (Utilities|FlowControl|Sequence
        (:then_0
          ;[1 1 1] 标记平台
          (if _hit
            (Utilities|IsValid _actor
              (:Is%20Valid
                (bind _platformref (Class|BPIPlatform|BPIGetPlatformRef(Message) _actor))
                (CallFunction|AddPlatformtoQueue _platformref)
                (Development|PrintString (Utilities|GetDisplayName _actor))))))
        (:then_1
          ;[1 1 1] 捡物品
          (if _hit_2
            (Utilities|IsValid _actor_2
              (:Is%20Valid
                (bind _keyref (Class|BPIKeys|BPIGetKeyRef(Message) _actor_2))
                (Default|PlayPickupSFX _keyref)
                (Utilities|Array|AddUnique (Variables|Interact|Getkeys) (Utilities|Struct|MakeST_key (Variables|/Game/_Game_/GamePaly/BP_/Others/BP_Keys.BP_Keys_C|GetLevel _keyref) (Variables|/Game/_Game_/GamePaly/BP_/Others/BP_Keys.BP_Keys_C|GetTexture _keyref)))
                (Actor|DestroyActor _actor_2)
                (Default|RefreshUI (Variables|UI|GetBackpackUI) (Variables|Interact|Getkeys))))))))))

(event Custom|Jump_State
  ;[1 1 1] IA_move
  (Character|Jump)
  (Variables|Movement|SetMovementState "NewEnumerator2")
  (switch Utilities|FlowControl|Switch|SwitchonE_MovementState (Variables|Movement|GetMovementState)
    (:NewEnumerator4
      (CallFunction|StopWalkSound)
      (Pawn|Input|AddMovementInput (Math|Vector|GetForwardVector (Variables|Default|GetDirection)) (Input|AxisValues|GetMove) true :!label _label))
    (:NewEnumerator0
      (CallFunction|PlayWalkSound :!label _label_2)
      (goto _label))
    (:NewEnumerator1
      (goto _label_2))
    (:NewEnumerator2
      (CallFunction|StopWalkSound)
      (Pawn|Input|AddMovementInput (Math|Vector|GetForwardVector (Variables|Default|GetDirection)) (Input|AxisValues|GetMove) true))))

(event Custom|ZoomCamera
  (params (Value :type Float%20%28double-precision%29))
  (bind _location (CallFunction|GetMouseLocationinMap))
  (bind _paintingviewlocation (Variables|摄像机|GetPaintingViewLocation))
  (bind (_x _y _z) (Math|Vector|BreakVector _location))
  (bind (_x_2 _y_2 _z_2) (Math|Vector|BreakVector _paintingviewlocation))
  ;[1 1 1] Zoom
  (if (< Value 0.0)
    (switch Utilities|FlowControl|Switch|SwitchonE_View (Variables|摄像机|GetView)
      (:NewEnumerator0
        (Variables|摄像机|SetPaintingView 1024.0)
        (Variables|摄像机|SetCameraLocation (Math|Vector|MakeVector (Math|Float|Clamp(Float) _x (- _x_2 5e+02) (+ _x_2 5e+02)) 0.0 (Math|Float|Clamp(Float) _z (- _z_2 3e+02) (+ _z_2 3e+02))))
        (Variables|摄像机|SetZooming true)))
    (else
      (Variables|摄像机|SetZooming false)
      (Variables|摄像机|SetPaintingView 2.4e+03))))

(event Custom|Fly
  (params (Value :type Float%20%28double-precision%29))
  ;[1 1 1] Fly
  (Sprite|SetFlipbook (Variables|Default|GetSprite) "/Game/_Game_/PlayerAnimation/Dream_Jump.Dream_Jump")
  (Pawn|Input|AddMovementInput (Math|Vector|MakeVector 0.0 0.0 Value) 1.0 false))

(event Input|EnhancedActionEvents|EnhancedInputActionIA_Move
  (params (ActionValue :type Float%20%28double-precision%29) (ElapsedSeconds :type Float%20%28double-precision%29) (TriggeredSeconds :type Float%20%28double-precision%29) (InputAction :type Input%20Action%20Object%20Reference :default "/Game/_Game_/GamePaly/Input/IA_Move.IA_Move"))
  ;[1 0.06189 0] 暂留
)

(event Input|EnhancedActionEvents|EnhancedInputActionIA_Jump
  (params (ActionValue :type Boolean) (ElapsedSeconds :type Float%20%28double-precision%29) (TriggeredSeconds :type Float%20%28double-precision%29) (InputAction :type Input%20Action%20Object%20Reference :default "/Game/_Game_/GamePaly/Input/IA_Jump.IA_Jump"))
  ;[1 0.06189 0] 暂留
)

(event Input|EnhancedActionEvents|EnhancedInputActionIA_Zoom
  (params (ActionValue :type Float%20%28double-precision%29) (ElapsedSeconds :type Float%20%28double-precision%29) (TriggeredSeconds :type Float%20%28double-precision%29) (InputAction :type Input%20Action%20Object%20Reference :default "/Game/_Game_/GamePaly/Input/IA_Zoom.IA_Zoom"))
  ;[1 0 0.03622] 暂留
  (CallFunction|ZoomCamera ActionValue))

(event Input|ActionEvents|InputActionPainting
  (params (Key :type Key%20Structure :default "None"))
  (:Pressed
    (CallFunction|PaintingEvent)))

(event Input|ActionEvents|InputActionSleep
  (params (Key :type Key%20Structure :default "None"))
  (:Pressed
    (CallFunction|Interact)))

(event Input|ActionEvents|InputActionJump
  (params (Key :type Key%20Structure :default "None"))
  (:Pressed
    (if (not (Variables|Input|GetIsFlying))
      (CallFunction|JumpState))))

(event Input|ActionEvents|InputActionTest
  (params (Key :type Key%20Structure :default "None"))
  ;[0 1 0.295] Test
  (:Pressed
    (Actor|GetActorOfClass "/Game/_Game_/GamePaly/BP_/Others/BP_Bridge.BP_Bridge_C")))

(event Input|AxisEvents|InputAxisMove
  (params (AxisValue :type Float%20%28single-precision%29))
  (CallFunction|Move AxisValue))

(event Input|AxisEvents|InputAxisZoom
  (params (AxisValue :type Float%20%28single-precision%29))
  ;[1 0 0.03622] 暂留
)

(event Input|AxisEvents|InputAxisFly
  (params (AxisValue :type Float%20%28single-precision%29)))

(event Custom|Reborn
  (bind _rebornui (Variables|UI|GetRebornUI))
  (bind _pc (Variables|PC|GetPC))
  (Audio|PlaySound2D "/Game/_Game_/Audio/SFX/character/hurt/SC_hurt.SC_hurt" 1.0 1.0 0.0 0 0)
  (Widget|SetVisibility _rebornui "Visible")
  (Input|SetInputModeUIOnly _pc _rebornui "DoNotLock" false)
  (Variables|/Script/Engine.PlayerController|SetbShowMouseCursor _pc true))

(event Custom|SetViewStateCalledByOthersBP
  (params (View :type E_View%20Enum :default "NewEnumerator0"))
  (Variables|摄像机|SetView View))

(event Custom|ReallyReborn
  (Transformation|SetActorLocation (+ (Variables|Default|GetSaveLocation) "0.000000,5.000000,0.000000") false false))

(event Custom|CreatBackpackUI
  (bind _returnvalue (UserInterface|CreateWidget "/Game/_Game_/GamePaly/UI/WB_Backpack.WB_Backpack_C" (Variables|PC|GetPC)))
  (bind _output_get (Variables|UI|SetBackpackUI _returnvalue))
  (UserInterface|Viewport|AddtoViewport _output_get 0)
  (bind _returnvalue_2 (UserInterface|CreateWidget "/Game/_Game_/GamePaly/UI/WB_Dream.WB_Dream_C" (Variables|PC|GetPC)))
  (bind _output_get_2 (Variables|UI|SetDream_UI _returnvalue_2))
  (UserInterface|Viewport|AddtoViewport _output_get_2 10)
  (bind _returnvalue_3 (UserInterface|CreateWidget "/Game/_Game_/GamePaly/UI/WB_GameOver.WB_GameOver_C" (Variables|PC|GetPC)))
  (bind _output_get_3 (Variables|UI|SetRebornUI _returnvalue_3))
  (UserInterface|Viewport|AddtoViewport _output_get_3 30)
  (Widget|SetVisibility _output_get_3 "Hidden"))

(fn ConstructionScript
  (Variables|/Script/Engine.CharacterMovementComponent|SetJumpZVelocity (Variables|Character|GetCharacterMovement) (Variables|Default|GetJumpSpeed)))

(fn OnRepMovementState
  (bind _returnvalue (Input|AxisValues|GetMove))
  (bind _movementstate (Variables|Movement|GetMovementState))
  (if (Math|Boolean|ORBoolean (Utilities|Enum|Equal(Enum) _movementstate "NewEnumerator0") (Utilities|Enum|Equal(Enum) _movementstate "NewEnumerator1") (!= _returnvalue 0.0))
    (Transformation|SetRelativeRotation (Variables|Default|GetSprite) (Math|Rotator|MakeRotator 0.0 0.0 (select (< _returnvalue 0.0) 1.8e+02 0.0)) false false))
  (Sprite|SetFlipbook (Variables|Default|GetSprite) (Utilities|Select :Index _movementstate :NewEnumerator4 "/Game/_Game_/PlayerAnimation/Dream_Idle.Dream_Idle" :NewEnumerator0 "/Game/_Game_/PlayerAnimation/Dream_Move.Dream_Move" :NewEnumerator1 "/Game/_Game_/PlayerAnimation/Dream_Move.Dream_Move" :NewEnumerator2 "/Game/_Game_/PlayerAnimation/Dream_Jump.Dream_Jump")))

(fn OnRepView
  (switch Utilities|FlowControl|Switch|SwitchonE_View (Variables|摄像机|GetView)
    (:NewEnumerator0
      (Sprite|SetFlipbook (Variables|Default|GetSprite) "/Game/_Game_/PlayerAnimation/Dream_Sleep.Dream_Sleep"))))

(fn CheckHit
  (params (Tag :type Name))
  (bind _pc (Variables|PC|GetPC))
  (bind _hitresult (Game|Player|GetHitResultUnderCursorbyChannel _pc "TraceTypeQuery1" true))
  (bind (_bblockinghit _binitialoverlap _time _distance _location _impactpoint _normal _impactnormal _physmat _hitactor) (Collision|BreakHitResult _hitresult))
  (if _bblockinghit
    (Utilities|IsValid _hitactor
      (:Is%20Valid
        (if (Actor|ActorHasTag _hitactor Tag)
          (return true _hitactor)
          (else
            _)))
      (:Is%20Not%20Valid
        _)))
  (return false 0))

(fn GetMouseLocationinMap
  (bind _pc (Variables|PC|GetPC))
  (bind _hitresult (Game|Player|GetHitResultUnderCursorbyChannel _pc "TraceTypeQuery1" true))
  (bind _location (Collision|BreakHitResult _hitresult))
  (bind (_x _y _z) (Math|Vector|BreakVector _location))
  (return (Math|Vector|MakeVector _x (.Y (Math|Vector|BreakVector (Variables|摄像机|GetPaintingViewLocation))) _z)))

(fn FindBackKeys
  (params (Keys :type Array%20of%20ST%20Key%20Structures) (index :type Integer) (DontRemove :type Boolean))
  (if (Utilities|Array|IsNotEmpty Keys)
    (for _array_element Keys
      (if (== (.index (Utilities|Struct|BreakST_key _array_element)) index)
        (if DontRemove
          _
          (else
            (Utilities|Array|RemoveItem Keys _array_element)
            (Default|RefreshUI (Variables|UI|GetBackpackUI) (Variables|Interact|Getkeys))))
        (return true)))
    (return false)
    (else
      (return false))))

(fn InSleep
  (Sprite|SetFlipbook (Variables|Default|GetSprite) "/Game/_Game_/PlayerAnimation/Dream_Sleep.Dream_Sleep")
  (Transformation|SetActorLocation (Variables|Default|GetSleeplocation) false false))

(fn PlayWalkSound
  (if (not (Variables|Input|GetIsFlying))
    (if (not (Variables|Default|GetPlayingWalkSFX))
      (Audio|Components|Audio|Play (Variables|Default|GetWalkSound) 0.0)
      (Variables|Default|SetPlayingWalkSFX true))))

(fn StopWalkSound
  (if (Variables|Default|GetPlayingWalkSFX)
    (Audio|Components|Audio|Stop (Variables|Default|GetWalkSound))
    (Variables|Default|SetPlayingWalkSFX false)))

(fn SoundsAboutDreamtoReality
  (bind _returnvalue (Actor|GetActorOfClass "/Game/_Game_/GamePaly/BP_/Others/BP_BackgroundMusic.BP_BackgroundMusic_C"))
  (Default|DreamtoReality _returnvalue)
  (bind _returnvalue_2 (Actor|GetActorOfClass "/Game/_Game_/GamePaly/BP_/Others/BP_BackgroudSFX.BP_BackgroudSFX_C"))
  (Default|StartPlaySFX _returnvalue_2))

(fn SoundsAboutRealitytoDream)

(fn AddPlatformtoQueue
  (params (NewBeChoosedPlatform :type BP%20Platform%20Object%20Reference%20%28by%20ref%29))
  (if (Utilities|Array|ContainsItem (Variables|Default|GetPlatformsRef) NewBeChoosedPlatform)
    (Default|NommalStateCBCBP NewBeChoosedPlatform)
    (Math|Integer|DecrementInt (Variables|Default|GetCurrentChooseplatformCount))
    (else
      (if (>= (Variables|Default|GetCurrentChooseplatformCount) (Variables|Default|GetMaxChoosePlatformCount))
        (Default|NommalStateCBCBP (Utilities|Array|Get(acopy) (Variables|Default|GetPlatformsRef)))
        (Utilities|Array|RemoveItem (Variables|Default|GetPlatformsRef) (Utilities|Array|Get(acopy) (Variables|Default|GetPlatformsRef)))
        (Utilities|Array|AddUnique (Variables|Default|GetPlatformsRef) NewBeChoosedPlatform)
        (else
          (Utilities|Array|AddUnique (Variables|Default|GetPlatformsRef) NewBeChoosedPlatform)
          (Math|Integer|IncrementInt (Variables|Default|GetCurrentChooseplatformCount)
            (:%20%20
              _))))
      (Default|BePaintingStateCalledbyCharacterBP NewBeChoosedPlatform))))

(fn BPIGetCharacterRef
  (return self))