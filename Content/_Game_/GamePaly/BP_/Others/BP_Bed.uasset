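; BP_Bed is an interactable bed that lets the player sleep.
; When an actor tagged Player enters its box, it fetches the character through an interface, enables sleeping, passes sleep and painting-view locations, sets the interact state and shows a prompt widget.
; Leaving the box disables sleeping and hides the widget.
; An interface function returns the bed itself as a reference.
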(event OnComponentBeginOverlap(Box)
  (params (OverlappedComponent :type Primitive%20Component%20Object%20Reference) (OtherActor :type Actor%20Object%20Reference) (OtherComp :type Primitive%20Component%20Object%20Reference) (OtherBodyIndex :type Integer) (bFromSweep :type Boolean) (SweepResult :type Hit%20Result%20Structure%20%28by%20ref%29))
  (if (Actor|ActorHasTag OtherActor "Player")
    (bind _characterref (Class|BPICharacter|BPIGetCharacterRef(Message) OtherActor))
    (Variables|/Game/_Game_/GamePaly/BP_/Player/BP_Character.BP_Character_C|SetCanSleep _characterref true)
    (Variables|/Game/_Game_/GamePaly/BP_/Player/BP_Character.BP_Character_C|SetPaintingViewLocation _characterref (Transformation|GetWorldLocation (Variables|Default|GetCameraLocation_Painting)))
    (Variables|/Game/_Game_/GamePaly/BP_/Player/BP_Character.BP_Character_C|SetSleeplocation _characterref (+ (Transformation|GetWorldLocation (Variables|Default|GetSleepLocation)) "0.000000,5.000000,0.000000"))
    (Variables|/Game/_Game_/GamePaly/BP_/Player/BP_Character.BP_Character_C|SetInteractState _characterref "NewEnumerator0")
    (Rendering|SetVisibility (Variables|Default|GetWidget) true false)))

(event OnComponentEndOverlap(Box)
  (params (OverlappedComponent :type Primitive%20Component%20Object%20Reference) (OtherActor :type Actor%20Object%20Reference) (OtherComp :type Primitive%20Component%20Object%20Reference) (OtherBodyIndex :type Integer))
  (if (Actor|ActorHasTag OtherActor "Player")
    (bind _characterref (Class|BPICharacter|BPIGetCharacterRef(Message) OtherActor))
    (Variables|/Game/_Game_/GamePaly/BP_/Player/BP_Character.BP_Character_C|SetCanSleep _characterref false)
    (Rendering|SetVisibility (Variables|Default|GetWidget) false false)))

(event EventBeginPlay
  (Rendering|SetVisibility (Variables|Default|GetWidget) false false))

(fn ConstructionScript)

(fn BPIGetBedRef
  (return self))