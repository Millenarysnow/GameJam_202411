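; Two-sided Paper2D door that teleports the player through, with three key indicators that external calls can hide individually or show all at once.
; Front and back overlap boxes show a prompt, register the door on the player character and record which side the player is on.
; TransPlayer_CBCBP teleports immediately from the back; from the front, the first call plays the opening flipbook and gate sound, and calls once open teleport.
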(event OnComponentBeginOverlap(Box_Enter)
  (params (OverlappedComponent :type Primitive%20Component%20Object%20Reference) (OtherActor :type Actor%20Object%20Reference) (OtherComp :type Primitive%20Component%20Object%20Reference) (OtherBodyIndex :type Integer) (bFromSweep :type Boolean) (SweepResult :type Hit%20Result%20Structure%20%28by%20ref%29))
  (if (Actor|ActorHasTag OtherActor "Player")
    (bind _characterref (Class|BPICharacter|BPIGetCharacterRef(Message) OtherActor))
    (Variables|/Game/_Game_/GamePaly/BP_/Player/BP_Character.BP_Character_C|SetLastDoorRef _characterref self)
    (Variables|/Game/_Game_/GamePaly/BP_/Player/BP_Character.BP_Character_C|SetinDoor _characterref true)
    (Variables|Default|Setinbackdoor false)
    (Rendering|SetVisibility (Variables|Default|GetInteract) true false)
    (Variables|/Game/_Game_/GamePaly/BP_/Player/BP_Character.BP_Character_C|SetInteractState _characterref "NewEnumerator5")))

(event OnComponentBeginOverlap(Out)
  (params (OverlappedComponent :type Primitive%20Component%20Object%20Reference) (OtherActor :type Actor%20Object%20Reference) (OtherComp :type Primitive%20Component%20Object%20Reference) (OtherBodyIndex :type Integer) (bFromSweep :type Boolean) (SweepResult :type Hit%20Result%20Structure%20%28by%20ref%29))
  (if (Actor|ActorHasTag OtherActor "Player")
    (bind _characterref (Class|BPICharacter|BPIGetCharacterRef(Message) OtherActor))
    (Variables|/Game/_Game_/GamePaly/BP_/Player/BP_Character.BP_Character_C|SetLastDoorRef _characterref self)
    (Variables|/Game/_Game_/GamePaly/BP_/Player/BP_Character.BP_Character_C|SetinDoor _characterref true)
    (Variables|Default|Setinbackdoor true)
    (Rendering|SetVisibility (Variables|Default|Getinteract2) true false)
    (Variables|/Game/_Game_/GamePaly/BP_/Player/BP_Character.BP_Character_C|SetInteractState _characterref "NewEnumerator5")))

(event OnComponentEndOverlap(Box_Enter)
  (params (OverlappedComponent :type Primitive%20Component%20Object%20Reference) (OtherActor :type Actor%20Object%20Reference) (OtherComp :type Primitive%20Component%20Object%20Reference) (OtherBodyIndex :type Integer))
  (if (Actor|ActorHasTag OtherActor "Player")
    (Rendering|SetVisibility (Variables|Default|GetInteract) false false)
    (bind _characterref (Class|BPICharacter|BPIGetCharacterRef(Message) OtherActor))
    (Variables|/Game/_Game_/GamePaly/BP_/Player/BP_Character.BP_Character_C|SetLastDoorRef _characterref 0)
    (Variables|/Game/_Game_/GamePaly/BP_/Player/BP_Character.BP_Character_C|SetinDoor _characterref false)))

(event OnComponentEndOverlap(Out)
  (params (OverlappedComponent :type Primitive%20Component%20Object%20Reference) (OtherActor :type Actor%20Object%20Reference) (OtherComp :type Primitive%20Component%20Object%20Reference) (OtherBodyIndex :type Integer))
  (if (Actor|ActorHasTag OtherActor "Player")
    (Rendering|SetVisibility (Variables|Default|Getinteract2) false false)
    (bind _characterref (Class|BPICharacter|BPIGetCharacterRef(Message) OtherActor))
    (Variables|/Game/_Game_/GamePaly/BP_/Player/BP_Character.BP_Character_C|SetLastDoorRef _characterref 0)
    (Variables|/Game/_Game_/GamePaly/BP_/Player/BP_Character.BP_Character_C|SetinDoor _characterref false)))

(event Custom|ShowKeys_CBCBP
  (params (index :type Integer))
  (Rendering|SetVisibility (Utilities|Array|Get(acopy) (Variables|Default|GetArray) index) false true))

(event Custom|ShowAllArrow_CBCBP
  (for _array_element (Variables|Default|GetArray)
    (Rendering|SetVisibility _array_element true true)))

(event Custom|TransPlayer_CBCBP
  (if (Variables|Default|Getinbackdoor)
    (Transformation|SetActorLocation (Game|Player|GetPlayerPawn 0) (+ (Transformation|GetWorldLocation (Variables|Default|Getoutlocation)) "0.000000,5.000000,0.000000") false false)
    (elif (Variables|Default|GetOpen)
      (Transformation|SetActorLocation (Game|Player|GetPlayerPawn 0) (+ (Transformation|GetWorldLocation (Variables|Default|GetEnterDoor_outlocation)) "0.000000,5.000000,0.000000") false false)
      (elif (not (Variables|Default|GetOpening))
        (Variables|Default|SetOpening true)
        (Sprite|SetFlipbook (Variables|Default|Getdoor) (Variables|Default|GetOpeningPaper))
        (Audio|Components|Audio|Play (Variables|Default|GetSC_rock_gate) 0.0)
        (Utilities|FlowControl|Delay (Class|PaperFlipbookComponent|GetFlipbookLength (Variables|Default|Getdoor)))
        (Sprite|SetFlipbook (Variables|Default|Getdoor) (Variables|Default|GetOpenEndingPaper))
        (Variables|Default|SetOpen true)))))

(fn ConstructionScript
  (Variables|Default|SetArray (Utilities|Array|MakeArray (Variables|Default|GetKey_Need1) (Variables|Default|GetKey_Need2) (Variables|Default|GetKey_Need3))))