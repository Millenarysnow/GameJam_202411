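; Child trap Blueprint, derived from a parent whose construction script it runs first, that lays out a configurable row of trap sprites.
; The construction script adds Count Paper2D sprite components, offset along X by multiples of Distance from the TrepSprite component's relative transform.
; Each copy uses the S_Trep sprite with collision disabled, and both the copies and the original TrepSprite are set invisible.
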(fn ConstructionScript
  (bind _trep_sprite (Variables|Default|GetTrep_Sprite))
  (bind _returnvalue (Transformation|GetRelativeTransform _trep_sprite))
  (bind (_x _y _z) (Math|Vector|BreakVector (.location _returnvalue)))
  (|CallParentFunction)
  (for _index (range 1 (Variables|Default|GetCount))
    (bind _returnvalue_2 (AddComponent|AddPaperSpriteComponent false (Math|Transform|MakeTransform (Math|Vector|MakeVector (+ _x (* _index (Variables|Default|GetDistance))) _y _z) (.rotation _returnvalue) (.scale _returnvalue))))
    (Rendering|Components|Sprite|SetSprite _returnvalue_2 "/Game/_Game_/Sprite/S_Trep.S_Trep")
    (Collision|SetCollisionEnabled _returnvalue_2 "NoCollision")
    (Rendering|SetVisibility _returnvalue_2 false false))
  (Rendering|SetVisibility (Variables|Default|GetTrep_Sprite) false false))