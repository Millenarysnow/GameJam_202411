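; Background ambience Blueprint that plays random bird and bug sounds from BeginPlay, with interface events to start and stop it.
; Two timer loops wait a short random delay, play a random clip, then reschedule when audio finishes.
; Stopping clears IsPlaying and mutes both audio components.
; Both loops play through and bind to BirdsSFXAudio, so BugsSFXAudio only receives volume changes.
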(event Custom|PlayBugsSFX
  (Variables|Default|SetIsPlaying true)
  (Utilities|Time|SetTimerbyEvent (delegate Custom|BugsCustomEvent) (Math|Random|RandomFloatinRange 2.0 5.0)))

(event Custom|BugsCustomEvent
  (if (Variables|Default|GetIsPlaying)
    (Audio|Components|Audio|SetSound (Variables|Default|GetBirdsSFX_Audio) (.OutItem (Utilities|Array|Random (Variables|Default|GetBugsSFX))))
    (Audio|Components|Audio|Play (Variables|Default|GetBirdsSFX_Audio) 0.0)
    (EventDispatchers|AssignOnAudioFinished (Variables|Default|GetBirdsSFX_Audio) (delegate Custom|OnBugsAudioFinished))))

(event Custom|StartPlaySFX
  ;[1 1 1] Interface
  (Audio|Components|Audio|SetVolumeMultiplier (Variables|Default|GetBirdsSFX_Audio) 1.0 :!class /Script/Engine.AudioComponent)
  (Audio|Components|Audio|SetVolumeMultiplier (Variables|Default|GetBugsSFX_Audio) 1.0 :!class /Script/Engine.AudioComponent)
  (CallFunction|PlayBirdsSFX)
  (CallFunction|PlayBugsSFX))

(event Custom|OnBugsAudioFinished
  (Utilities|Time|SetTimerbyEvent (delegate Custom|BugsCustomEvent) (Math|Random|RandomFloatinRange 2.0 5.0)))

(event Custom|StopPlaySFX
  ;[1 1 1] Interface
  (Variables|Default|SetIsPlaying false)
  (Audio|Components|Audio|SetVolumeMultiplier (Variables|Default|GetBirdsSFX_Audio) 0.0 :!class /Script/Engine.AudioComponent)
  (Audio|Components|Audio|SetVolumeMultiplier (Variables|Default|GetBugsSFX_Audio) 0.0 :!class /Script/Engine.AudioComponent))

(event Custom|PlayBirdsSFX
  (Variables|Default|SetIsPlaying true)
  (Utilities|Time|SetTimerbyEvent (delegate Custom|BirdsCustomEvent) (Math|Random|RandomFloatinRange 2.0 5.0)))

(event Custom|BirdsCustomEvent
  (if (Variables|Default|GetIsPlaying)
    (Audio|Components|Audio|SetSound (Variables|Default|GetBirdsSFX_Audio) (.OutItem (Utilities|Array|Random (Variables|Default|GetBirdsSFX))))
    (Audio|Components|Audio|Play (Variables|Default|GetBirdsSFX_Audio) 0.0)
    (EventDispatchers|AssignOnAudioFinished (Variables|Default|GetBirdsSFX_Audio) (delegate Custom|OnBirdsAudioFinished))))

(event Custom|OnBirdsAudioFinished
  (Utilities|Time|SetTimerbyEvent (delegate Custom|BirdsCustomEvent) (Math|Random|RandomFloatinRange 2.0 5.0)))

(event EventBeginPlay
  ;[1 1 1] BeginPlay
  (CallFunction|StartPlaySFX))

(fn ConstructionScript)