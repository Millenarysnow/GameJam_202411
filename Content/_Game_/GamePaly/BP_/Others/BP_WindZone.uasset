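; BP_WindZone is a box trigger volume that lets the player fly while inside it.
; Begin and end overlap on Player-tagged actors fetch the character through a BPI interface and update its TouchWindZoneNum counter.
; SwitchCanFly is called only on entering the first zone and leaving the last, so overlapping zones do not toggle flight off early.
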(event OnComponentBeginOverlap(Box)
  (params (OverlappedComponent :type Primitive%20Component%20Object%20Reference) (OtherActor :type Actor%20Object%20Reference) (OtherComp :type Primitive%20Component%20Object%20Reference) (OtherBodyIndex :type Integer) (bFromSweep :type Boolean) (SweepResult :type Hit%20Result%20Structure%20%28by%20ref%29))
  (if (Actor|ActorHasTag OtherActor "Player")
    (bind _characterref (Class|BPICharacter|BPIGetCharacterRef(Message) OtherActor))
    (if (< (Variables|/Game/_Game_/GamePaly/BP_/Player/BP_Character.BP_Character_C|GetTouchWindZoneNum _characterref) 1)
      (Default|SwitchCanFly _characterref))
    (Variables|/Game/_Game_/GamePaly/BP_/Player/BP_Character.BP_Character_C|SetTouchWindZoneNum _characterref (+ (Variables|/Game/_Game_/GamePaly/BP_/Player/BP_Character.BP_Character_C|GetTouchWindZoneNum _characterref) 1))))

(event OnComponentEndOverlap(Box)
  (params (OverlappedComponent :type Primitive%20Component%20Object%20Reference) (OtherActor :type Actor%20Object%20Reference) (OtherComp :type Primitive%20Component%20Object%20Reference) (OtherBodyIndex :type Integer))
  (if (Actor|ActorHasTag OtherActor "Player")
    (bind _characterref (Class|BPICharacter|BPIGetCharacterRef(Message) OtherActor))
    (if (< (Variables|/Game/_Game_/GamePaly/BP_/Player/BP_Character.BP_Character_C|GetTouchWindZoneNum _characterref) 2)
      (Default|SwitchCanFly _characterref))
    (Variables|/Game/_Game_/GamePaly/BP_/Player/BP_Character.BP_Character_C|SetTouchWindZoneNum _characterref (- (Variables|/Game/_Game_/GamePaly/BP_/Player/BP_Character.BP_Character_C|GetTouchWindZoneNum _characterref) 1))))

(fn ConstructionScript)