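; Menu music Blueprint that sequences two audio components, Chord1 and Chord2, in a repeating pattern.
; Each component's OnAudioFinished event triggers the next playback, with a counter making Chord1 play twice before Chord2 plays once and hands back to Chord1.
; The graph contains no initial Play call, only these finish-event handlers.
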(event OnAudioFinished(Audio_Chord1)
  (Variables|Default|SetChord1Times (+ (Variables|Default|GetChord1Times) 1))
  (if (>= (Variables|Default|GetChord1Times) 2)
    (Variables|Default|SetChord1Times 0)
    (Audio|Components|Audio|Play (Variables|Default|GetAudio_Chord2) 0.0)
    (else
      (Audio|Components|Audio|Play (Variables|Default|GetAudio_Chord1) 0.0))))

(event OnAudioFinished(Audio_Chord2)
  (Audio|Components|Audio|Play (Variables|Default|GetAudio_Chord1) 0.0))

(fn ConstructionScript)