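; BP_WinDoor is a level exit actor that wins the game when the player reaches it holding the required key.
; Its Box overlap checks for the Player tag, gets the character through an interface message and searches its keys for index 7 without removing it.
; If found, Win shows the WB_Win widget with the mouse cursor and UI-only input.
; Otherwise it calls NoStar, which is currently empty.
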(event OnComponentBeginOverlap(Box)
  (params (OverlappedComponent :type Primitive%20Component%20Object%20Reference) (OtherActor :type Actor%20Object%20Reference) (OtherComp :type Primitive%20Component%20Object%20Reference) (OtherBodyIndex :type Integer) (bFromSweep :type Boolean) (SweepResult :type Hit%20Result%20Structure%20%28by%20ref%29))
  (if (Actor|ActorHasTag OtherActor "Player")
    (bind _characterref (Class|BPICharacter|BPIGetCharacterRef(Message) OtherActor))
    (if (Default|FindBackKeys _characterref (Variables|/Game/_Game_/GamePaly/BP_/Player/BP_Character.BP_Character_C|Getkeys _characterref) 7 true)
      (CallFunction|Win)
      (else
        (CallFunction|NoStar)))))

(event Custom|Win
  (bind _returnvalue (Game|GetPlayerController 0))
  (bind _returnvalue_2 (UserInterface|CreateWidget "/Game/_Game_/GamePaly/UI/WB_Win.WB_Win_C" _returnvalue))
  (UserInterface|Viewport|AddtoViewport _returnvalue_2 0)
  (Variables|/Script/Engine.PlayerController|SetbShowMouseCursor _returnvalue true)
  (Input|SetInputModeUIOnly _returnvalue _returnvalue_2 "DoNotLock" false))

(event Custom|NoStar)

(event EventBeginPlay)

(event Collision|EventActorBeginOverlap
  (params (OtherActor :type Actor%20Object%20Reference)))

(event EventTick
  (params (DeltaSeconds :type Float%20%28single-precision%29)))

(fn ConstructionScript)