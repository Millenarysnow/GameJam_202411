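; BP_Door01 is a key-locked Paper2D flipbook door that teleports the player between an entrance and an exit.
; Overlap boxes on each side show interact prompts and register the door with the character through an interface.
; On the character's interact call, a key opens the door with animation and sound; later interactions teleport the player.
; Entering saves the camera border and root locations before moving them, and returning restores them.
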(event OnComponentBeginOverlap(Box_Enter)
  (params (OverlappedComponent :type Primitive%20Component%20Object%20Reference) (OtherActor :type Actor%20Object%20Reference) (OtherComp :type Primitive%20Component%20Object%20Reference) (OtherBodyIndex :type Integer) (bFromSweep :type Boolean) (SweepResult :type Hit%20Result%20Structure%20%28by%20ref%29))
  (if (Actor|ActorHasTag OtherActor "Player")
    (bind _characterref (Class|BPICharacter|BPIGetCharacterRef(Message) OtherActor))
    (Variables|/Game/_Game_/GamePaly/BP_/Player/BP_Character.BP_Character_C|SetDoorRef _characterref self)
    (Variables|/Game/_Game_/GamePaly/BP_/Player/BP_Character.BP_Character_C|SetinDoor _characterref true)
    (Variables|Default|Setinbackdoor false)
    (Rendering|SetVisibility (Variables|Default|GetInteract) true false)
    (Variables|/Game/_Game_/GamePaly/BP_/Player/BP_Character.BP_Character_C|SetInteractState _characterref "NewEnumerator1")))

(event OnComponentEndOverlap(Box_Enter)
  (params (OverlappedComponent :type Primitive%20Component%20Object%20Reference) (OtherActor :type Actor%20Object%20Reference) (OtherComp :type Primitive%20Component%20Object%20Reference) (OtherBodyIndex :type Integer))
  (if (Actor|ActorHasTag OtherActor "Player")
    (Rendering|SetVisibility (Variables|Default|GetInteract) false false)
    (bind _characterref (Class|BPICharacter|BPIGetCharacterRef(Message) OtherActor))
    (Variables|/Game/_Game_/GamePaly/BP_/Player/BP_Character.BP_Character_C|SetDoorRef _characterref 0)
    (Variables|/Game/_Game_/GamePaly/BP_/Player/BP_Character.BP_Character_C|SetinDoor _characterref false)))

(event OnComponentBeginOverlap(Out)
  (params (OverlappedComponent :type Primitive%20Component%20Object%20Reference) (OtherActor :type Actor%20Object%20Reference) (OtherComp :type Primitive%20Component%20Object%20Reference) (OtherBodyIndex :type Integer) (bFromSweep :type Boolean) (SweepResult :type Hit%20Result%20Structure%20%28by%20ref%29))
  (if (Actor|ActorHasTag OtherActor "Player")
    (bind _characterref (Class|BPICharacter|BPIGetCharacterRef(Message) OtherActor))
    (Variables|/Game/_Game_/GamePaly/BP_/Player/BP_Character.BP_Character_C|SetDoorRef _characterref self)
    (Variables|/Game/_Game_/GamePaly/BP_/Player/BP_Character.BP_Character_C|SetinDoor _characterref true)
    (Variables|Default|Setinbackdoor true)
    (Rendering|SetVisibility (Variables|Default|Getinteract2) true false)
    (Variables|/Game/_Game_/GamePaly/BP_/Player/BP_Character.BP_Character_C|SetInteractState _characterref "NewEnumerator1")))

(event OnComponentEndOverlap(Out)
  (params (OverlappedComponent :type Primitive%20Component%20Object%20Reference) (OtherActor :type Actor%20Object%20Reference) (OtherComp :type Primitive%20Component%20Object%20Reference) (OtherBodyIndex :type Integer))
  (if (Actor|ActorHasTag OtherActor "Player")
    (Rendering|SetVisibility (Variables|Default|Getinteract2) false false)
    (bind _characterref (Class|BPICharacter|BPIGetCharacterRef(Message) OtherActor))
    (Variables|/Game/_Game_/GamePaly/BP_/Player/BP_Character.BP_Character_C|SetDoorRef _characterref 0)
    (Variables|/Game/_Game_/GamePaly/BP_/Player/BP_Character.BP_Character_C|SetinDoor _characterref false)))

(event Custom|PlayKeyUsedSFX
  (Audio|PlaySound2D (Variables|Default|GetItemUsedSound) 1.0 1.0 0.0 0 0))

(event Custom|interact_CalledByCharacterBP
  (params (have :type Boolean))
  (bind _out_cameralocation (Variables|Default|GetOut_CameraLocation))
  (bind _returnvalue (Transformation|GetWorldLocation _out_cameralocation))
  (if (Variables|Default|Getinbackdoor)
    (CallFunction|TransbackPlayer)
    (elif (Variables|Default|GetOpen)
      (bind _characterref (Class|BPICharacter|BPIGetCharacterRef(Message) (Game|Player|GetPlayerPawn 0)))
      (Variables|Default|SetEnterDoor%20Border%20Location (Variables|/Game/_Game_/GamePaly/BP_/Player/BP_Character.BP_Character_C|GetCameraBorderLocation _characterref))
      (Variables|Default|SetCamera%20Root%20Location (Variables|/Game/_Game_/GamePaly/BP_/Player/BP_Character.BP_Character_C|GetCameraRootLocation _characterref))
      (Variables|/Game/_Game_/GamePaly/BP_/Player/BP_Character.BP_Character_C|SetCameraBorderLocation _characterref _returnvalue)
      (Variables|/Game/_Game_/GamePaly/BP_/Player/BP_Character.BP_Character_C|SetCameraRootLocation _characterref _returnvalue)
      (Transformation|SetActorLocation (Game|Player|GetPlayerPawn 0) (+ (Transformation|GetWorldLocation (Variables|Default|Getoutlocation)) "0.000000,5.000000,0.000000") false false)
      (elif have
        (CallFunction|PlayKeyUsedSFX)
        (Sprite|SetFlipbook (Variables|Default|Getdoor) (Variables|Default|GetOpeningPaper))
        (Audio|Components|Audio|Play (Variables|Default|GetAudio) 0.0)
        (Utilities|FlowControl|Delay (Class|PaperFlipbookComponent|GetFlipbookLength (Variables|Default|Getdoor)))
        (Sprite|SetFlipbook (Variables|Default|Getdoor) (Variables|Default|GetOpenEndingPaper))
        (Variables|Default|SetOpen true)
        (Rendering|SetVisibility (Variables|Default|GetKey_Need) false true)))))

(event Custom|Transback_Player_
  (Transformation|SetActorLocation (Game|Player|GetPlayerPawn 0) (+ (Transformation|GetWorldLocation (Variables|Default|GetEnterDoor_outlocation)) "0.000000,5.000000,0.000000") false false)
  (bind _characterref (Class|BPICharacter|BPIGetCharacterRef(Message) (Game|Player|GetPlayerPawn 0)))
  (Variables|/Game/_Game_/GamePaly/BP_/Player/BP_Character.BP_Character_C|SetCameraBorderLocation _characterref (Variables|Default|GetEnterDoor%20Border%20Location))
  (Variables|/Game/_Game_/GamePaly/BP_/Player/BP_Character.BP_Character_C|SetCameraRootLocation _characterref (Variables|Default|GetCamera%20Root%20Location)))

(event EventBeginPlay
  (|CallParentFunction))

(fn ConstructionScript
  (|CallParentFunction))