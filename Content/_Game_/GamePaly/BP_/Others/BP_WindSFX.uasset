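; BP_WindSFX is a trigger-zone actor that plays wind sound while the player is inside its box volume.
; Overlap events on SFX_Zone_Box check for the Player tag, calling PlayWindSFX on entry and StopWindSFX on exit.
; Playback starts the first audio component, then the second after a fixed delay to layer them; stopping calls a zero-duration FadeOut on both without cancelling that pending delay.
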(event OnComponentBeginOverlap(SFX_Zone_Box)
  (params (OverlappedComponent :type Primitive%20Component%20Object%20Reference) (OtherActor :type Actor%20Object%20Reference) (OtherComp :type Primitive%20Component%20Object%20Reference) (OtherBodyIndex :type Integer) (bFromSweep :type Boolean) (SweepResult :type Hit%20Result%20Structure%20%28by%20ref%29))
  (if (Actor|ActorHasTag OtherActor "Player")
    (CallFunction|PlayWindSFX)))

(event OnComponentEndOverlap(SFX_Zone_Box)
  (params (OverlappedComponent :type Primitive%20Component%20Object%20Reference) (OtherActor :type Actor%20Object%20Reference) (OtherComp :type Primitive%20Component%20Object%20Reference) (OtherBodyIndex :type Integer))
  (if (Actor|ActorHasTag OtherActor "Player")
    (CallFunction|StopWindSFX)))

(event Custom|PlayWindSFX
  (Audio|Components|Audio|Play (Variables|Default|GetAudio1) 0.0)
  (Utilities|FlowControl|Delay 6.0)
  (Audio|Components|Audio|Play (Variables|Default|GetAudio2) 0.0))

(event Custom|StopWindSFX
  (Audio|Components|Audio|FadeOut (Variables|Default|GetAudio1) 0.0 0.0 "Linear" :!class /Script/Engine.AudioComponent)
  (Audio|Components|Audio|FadeOut (Variables|Default|GetAudio2) 0.0 0.0 "Linear" :!class /Script/Engine.AudioComponent))

(fn ConstructionScript)