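; BP_Door is a door that moves the player to its exit point when they walk into it while it is open.
; Overlapping Box_Enter with the Opening flag set teleports any actor tagged Player to the Out component's world location.
; It then gets the character reference from player pawn 0 through an interface call and sets its CameraBorderLocation to the exit plus a transfer offset.
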(event OnComponentBeginOverlap(Box_Enter)
  (params (OverlappedComponent :type Primitive%20Component%20Object%20Reference) (OtherActor :type Actor%20Object%20Reference) (OtherComp :type Primitive%20Component%20Object%20Reference) (OtherBodyIndex :type Integer) (bFromSweep :type Boolean) (SweepResult :type Hit%20Result%20Structure%20%28by%20ref%29))
  (bind _out (Variables|Default|GetOut))
  (bind _returnvalue (Transformation|GetWorldLocation _out))
  (if (Variables|Default|GetOpening)
    (if (Actor|ActorHasTag OtherActor "Player")
      (Transformation|SetActorLocation OtherActor _returnvalue false false)
      (bind _characterref (Class|BPICharacter|BPIGetCharacterRef(Message) (Game|Player|GetPlayerPawn 0)))
      (Variables|/Game/_Game_/GamePaly/BP_/Player/BP_Character.BP_Character_C|SetCameraBorderLocation _characterref (+ _returnvalue (Variables|Default|GetTrasferOffest))))))

(fn ConstructionScript)