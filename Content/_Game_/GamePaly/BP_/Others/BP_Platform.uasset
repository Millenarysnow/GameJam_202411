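; BP_Platform is a platform that the character Blueprint can show, hide or highlight, starting without collision.
; Showing enables query and physics collision with the platform material, while hiding disables collision and applies the M_CantBeSee material.
; The painting and normal state events swap only the Cube's material, leaving collision untouched.
; An interface function returns a self reference so other Blueprints can get the platform.
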(event Custom|ShowPlatform_CalledByCharacterBP
  (bind _cube (Variables|Default|GetCube))
  (Collision|SetCollisionEnabled _cube "QueryAndPhysics")
  (Rendering|Material|SetMaterial _cube 0 "/Game/_Game_/Material/M_Platform.M_Platform"))

(event Custom|HidePlatform_CalledByCharacterBP
  (bind _cube (Variables|Default|GetCube))
  (Collision|SetCollisionEnabled _cube "NoCollision")
  (Rendering|Material|SetMaterial _cube 0 "/Game/_Game_/Material/M_CantBeSee.M_CantBeSee"))

(event Custom|ShowAll
  (bind _cube (Variables|Default|GetCube))
  (Collision|SetCollisionEnabled _cube "QueryAndPhysics")
  (Rendering|Material|SetMaterial _cube 0 "/Game/_Game_/Material/M_Platform.M_Platform"))

(event Custom|BePaintingState_CalledByCharacterBP
  (Rendering|Material|SetMaterial (Variables|Default|GetCube) 0 "/Game/_Game_/Material/M_CanSee.M_CanSee"))

(event Custom|NommalState_CBCBP
  (Rendering|Material|SetMaterial (Variables|Default|GetCube) 0 "/Game/_Game_/Material/M_Platform.M_Platform"))

(event EventBeginPlay
  (Collision|SetCollisionEnabled (Variables|Default|GetCube) "NoCollision"))

(fn ConstructionScript)

(fn BPIGetPlatformRef
  (return self))