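; BP_Tool is a tool actor that the player can pick up.
; On begin play it passes its image to a key widget through an interface.
; Box overlaps with Player-tagged actors set or clear the character's pickup flag and tool reference through an interface, also setting the interact state on entry.
; Both overlap events set Widget1 visible, and the pickup and used SFX events are empty.
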(event OnComponentBeginOverlap(Box)
  (params (OverlappedComponent :type Primitive%20Component%20Object%20Reference) (OtherActor :type Actor%20Object%20Reference) (OtherComp :type Primitive%20Component%20Object%20Reference) (OtherBodyIndex :type Integer) (bFromSweep :type Boolean) (SweepResult :type Hit%20Result%20Structure%20%28by%20ref%29))
  (if (Actor|ActorHasTag OtherActor "Player")
    (bind _characterref (Class|BPICharacter|BPIGetCharacterRef(Message) OtherActor))
    (Variables|/Game/_Game_/GamePaly/BP_/Player/BP_Character.BP_Character_C|SetInteractState _characterref "NewEnumerator4")
    (Variables|/Game/_Game_/GamePaly/BP_/Player/BP_Character.BP_Character_C|SetCanPick _characterref true)
    (Variables|/Game/_Game_/GamePaly/BP_/Player/BP_Character.BP_Character_C|SetTool _characterref self)
    (Rendering|SetVisibility (Variables|Default|GetWidget1) true false)))

(event OnComponentEndOverlap(Box)
  (params (OverlappedComponent :type Primitive%20Component%20Object%20Reference) (OtherActor :type Actor%20Object%20Reference) (OtherComp :type Primitive%20Component%20Object%20Reference) (OtherBodyIndex :type Integer))
  (if (Actor|ActorHasTag OtherActor "Player")
    (bind _characterref (Class|BPICharacter|BPIGetCharacterRef(Message) OtherActor))
    (Variables|/Game/_Game_/GamePaly/BP_/Player/BP_Character.BP_Character_C|SetCanPick _characterref false)
    (Variables|/Game/_Game_/GamePaly/BP_/Player/BP_Character.BP_Character_C|SetTool _characterref 0)
    (Rendering|SetVisibility (Variables|Default|GetWidget1) true false)))

(event Custom|PlayPickupSFX)

(event Custom|PlayUsedSFX)

(event EventBeginPlay
  (bind _wb_keyref (Class|BPIKeyUI|BPIGetKeyRef(Message) (UserInterface|GetWidget (Variables|Default|GetWidget))))
  (Default|SetImage _wb_keyref (Variables|Default|GetImage)))

(fn ConstructionScript)