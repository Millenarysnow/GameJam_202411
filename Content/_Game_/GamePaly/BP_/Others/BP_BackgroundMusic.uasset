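; Background music actor that crossfades between dream and reality tracks when the game switches between the two worlds.
; Both audio components start playing together in the construction script.
; DreamToReality and RealityToDream each play a 2D transition cue, then call a function that restarts the matching timeline, whose Music curve drives inverse volume multipliers on the two tracks.
; SwitchMusic is an empty stub.
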(event Custom|DreamToReality
  (Audio|PlaySound2D "/Game/_Game_/Audio/SFX/interaction/alter/SC_dreamOut.SC_dreamOut" 1.0 1.0 0.0 0 0)
  (CallFunction|SwitchMusicDreamtoReality))

(event Custom|RealityToDream
  (Audio|PlaySound2D "/Game/_Game_/Audio/SFX/interaction/alter/SC_dreamIn.SC_dreamIn" 1.0 1.0 0.0 0 0)
  (CallFunction|SwitchMusicRealitytoDream))

(fn ConstructionScript
  (Utilities|FlowControl|Sequence
    (:then_0
      (Audio|Components|Audio|Play (Variables|Default|GetAudio_Dream) 0.0))
    (:then_1
      (Audio|Components|Audio|Play (Variables|Default|GetAudio_Reality) 0.0))))

(fn SwitchMusicDreamtoReality
  (Components|Timeline|PlayfromStart (Variables|Default|GetDToR)))

(fn SwitchMusicRealitytoDream
  (Components|Timeline|PlayfromStart (Variables|Default|GetRToD)))

(fn SwitchMusic
  (params (Status :type E_View%20Enum :default "NewEnumerator0"))
  (return))