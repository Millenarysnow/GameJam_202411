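; BP_Traps is a trap actor that triggers Reborn on the player character when an actor tagged "player" overlaps its Box.
; The character reference comes through an interface call on player pawn 0, not from the overlapping actor.
; Events switch the mesh between its default and can't-be-seen materials and toggle custom depth for masking.
; An interface function returns the trap's own reference.
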(event OnComponentBeginOverlap(Box)
  (params (OverlappedComponent :type Primitive%20Component%20Object%20Reference) (OtherActor :type Actor%20Object%20Reference) (OtherComp :type Primitive%20Component%20Object%20Reference) (OtherBodyIndex :type Integer) (bFromSweep :type Boolean) (SweepResult :type Hit%20Result%20Structure%20%28by%20ref%29))
  (CallFunction|PlayerCollision OtherActor))

(event Custom|SetMaterial
  (params (canSee :type Boolean))
  (Rendering|Material|SetMaterial (Variables|Default|GetStaticMesh) 0 (select canSee "/Engine/EngineMaterials/DefaultMaterial.DefaultMaterial" "/Game/_Game_/Material/M_CantBeSee.M_CantBeSee")))

(event Custom|BeMasked
  (params (BeMasked :type Boolean))
  (Rendering|SetRenderCustomDepth (Variables|Default|GetStaticMesh) BeMasked))

(fn ConstructionScript)

(fn PlayerCollision
  (params (self2 :type Actor%20Object%20Reference))
  (if (Actor|ActorHasTag self2 "player")
    (bind _characterref (Class|BPICharacter|BPIGetCharacterRef(Message) (Game|Player|GetPlayerPawn 0)))
    (Default|Reborn _characterref)))

(fn BPIGetTrapRef
  (return self))