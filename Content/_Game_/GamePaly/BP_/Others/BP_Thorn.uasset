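; BP_Thorn is a thorn obstacle that reacts to overlaps on its Box component and then removes itself.
; An overlap passes the other actor to PlayerCollision, then destroys the thorn after a short delay, with no filter in the event itself.
; A separate Destory function, not called in this graph, destroys the thorn immediately when the supplied actor is tagged "floor".
; Construction runs the parent script and prints a debug string.
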(event OnComponentBeginOverlap(Box)
  (params (OverlappedComponent :type Primitive%20Component%20Object%20Reference) (OtherActor :type Actor%20Object%20Reference) (OtherComp :type Primitive%20Component%20Object%20Reference) (OtherBodyIndex :type Integer) (bFromSweep :type Boolean) (SweepResult :type Hit%20Result%20Structure%20%28by%20ref%29))
  (CallFunction|PlayerCollision OtherActor)
  (Utilities|FlowControl|Delay 2.0)
  (Actor|DestroyActor))

(fn ConstructionScript
  (|CallParentFunction)
  (Development|PrintString "construction"))

(fn Destory
  (params (self2 :type Actor%20Object%20Reference))
  (if (Actor|ActorHasTag self2 "floor")
    (Development|PrintString "destroy" true true "(R=1.000000,G=0.000000,B=0.021455,A=1.000000)")
    (Actor|DestroyActor)))