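; BP_TransDoor is a teleport door that moves the player to its TargetLocation point.
; Overlapping its Box with a Player-tagged actor sets the character's in-door flag, door reference and interact state, and shows a Widget; leaving clears the flag and reference and hides the Widget.
; The TransPlayer event, not triggered within this Blueprint, places player pawn 0 slightly offset from the target and updates its camera root location to below that point.
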(event OnComponentBeginOverlap(Box)
  (params (OverlappedComponent :type Primitive%20Component%20Object%20Reference) (OtherActor :type Actor%20Object%20Reference) (OtherComp :type Primitive%20Component%20Object%20Reference) (OtherBodyIndex :type Integer) (bFromSweep :type Boolean) (SweepResult :type Hit%20Result%20Structure%20%28by%20ref%29))
  (if (Actor|ActorHasTag OtherActor "Player")
    (bind _characterref (Class|BPICharacter|BPIGetCharacterRef(Message) OtherActor))
    (Variables|/Game/_Game_/GamePaly/BP_/Player/BP_Character.BP_Character_C|SetInTransDoor _characterref true)
    (Variables|/Game/_Game_/GamePaly/BP_/Player/BP_Character.BP_Character_C|SetTransDoorRef _characterref self)
    (Variables|/Game/_Game_/GamePaly/BP_/Player/BP_Character.BP_Character_C|SetInteractState _characterref "NewEnumerator2")
    (Rendering|SetVisibility (Variables|Default|GetWidget) true false)))

(event OnComponentEndOverlap(Box)
  (params (OverlappedComponent :type Primitive%20Component%20Object%20Reference) (OtherActor :type Actor%20Object%20Reference) (OtherComp :type Primitive%20Component%20Object%20Reference) (OtherBodyIndex :type Integer))
  (if (Actor|ActorHasTag OtherActor "Player")
    (bind _characterref (Class|BPICharacter|BPIGetCharacterRef(Message) OtherActor))
    (Variables|/Game/_Game_/GamePaly/BP_/Player/BP_Character.BP_Character_C|SetInTransDoor _characterref false)
    (Variables|/Game/_Game_/GamePaly/BP_/Player/BP_Character.BP_Character_C|SetTransDoorRef _characterref 0)
    (Rendering|SetVisibility (Variables|Default|GetWidget) false false)))

(event Custom|TransPlayer
  (bind _targetlocation_ (Variables|Default|GetTargetLocation_))
  (bind _returnvalue (Transformation|GetWorldLocation _targetlocation_))
  (bind _characterref (Class|BPICharacter|BPIGetCharacterRef(Message) (Game|Player|GetPlayerPawn 0)))
  (Transformation|SetActorLocation _characterref (+ _returnvalue "0.000000,5.000000,0.000000") false false)
  (Variables|/Game/_Game_/GamePaly/BP_/Player/BP_Character.BP_Character_C|SetCameraRootLocation _characterref (- _returnvalue "0.000000,0.000000,100.000000")))

(fn ConstructionScript)